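; Test overworld character that moves under point gravity centred on the world origin.
; BeginPlay sets that gravity through the Ninja character movement component.
; Movement axes project the camera's up and right vectors onto the ground plane, found by a short debug-drawn trace along the capsule's down direction.
; Tick also consumes the movement component's input vector every frame.
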(event `self.ReceiveBeginPlay`
  (`self.Set Gravity`))

(event `self.ReceiveTick`
  (params (DeltaSeconds :type "Float (single-precision)"))
  (`PawnMovementComponent.ConsumeInputVector` (`self.CharacterMovement`)))

(event `InputAxis|Axis_Move_UpDown`
  (params (AxisValue :type "Float (single-precision)"))
  (`self.AddMovementInput` (`KismetMathLibrary.ProjectVectorOnToPlane` (`SceneComponent.GetUpVector` (`self.Camera`)) (`.ImpactNormal` (`self.Get Ground`))) AxisValue))

(event `InputAxis|Axis_Move_LeftRight`
  (params (AxisValue :type "Float (single-precision)"))
  (`self.AddMovementInput` (`KismetMathLibrary.ProjectVectorOnToPlane` (`SceneComponent.GetRightVector` (`self.Camera`)) (`.ImpactNormal` (`self.Get Ground`))) AxisValue))

(fn `Get Ground`
  (returns (OutHit :type "HitResult Structure") (ImpactNormal :type "Vector Structure"))
  (bind _returnvalue (`self.K2_GetActorLocation`))
  (bind _outhit (`KismetSystemLibrary.LineTraceSingle` :`Start` _returnvalue :`End` (+ _returnvalue (* (`SceneComponent.GetUpVector` (`self.CapsuleComponent`)) -32.0)) :`TraceChannel` "TraceTypeQuery1" :`DrawDebugType` "ForOneFrame"))
  (return _outhit (`.ImpactNormal` (`GameplayStatics.BreakHitResult` _outhit))))

(fn `Set Gravity`
  (bind _asninja_character_movement_component (cast `NinjaCharacterMovementComponent` (`self.CharacterMovement`)))
  (`NinjaCharacterMovementComponent.SetPointGravityDirection` _asninja_character_movement_component (0.0 0.0 0.0)))

(fn `UserConstructionScript`)